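; BP_Human is a human character that turns into a flung ragdoll and disappears when it takes any damage.
; The first hit switches the mesh to simulated ragdoll physics and makes both mesh and capsule ignore Pawn and Camera channels.
; It launches the mesh along the damage causer's normalized world location, not a relative hit direction, then destroys the actor after a short delay.
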(event `self.ReceiveAnyDamage`
  (params (Damage :type "Float (single-precision)") (DamageType :type "DamageType Object Reference") (InstigatedBy :type "Controller Object Reference") (DamageCauser :type "Actor Object Reference"))
  (bind _mesh (`self.Mesh`))
  (bind _capsulecomponent (`self.CapsuleComponent`))
  (`/Engine/EditorBlueprintResources/StandardMacros.DoOnce` false
    (:`Completed`
      (`PrimitiveComponent.SetCollisionProfileName` _mesh "Ragdoll" true)
      (`PrimitiveComponent.SetCollisionResponseToChannel` _mesh "ECC_Pawn" "ECR_Ignore")
      (`PrimitiveComponent.SetCollisionResponseToChannel` _mesh "ECC_Camera" "ECR_Ignore")
      (`PrimitiveComponent.SetSimulatePhysics` _mesh true)
      (`PrimitiveComponent.SetCollisionResponseToChannel` _capsulecomponent "ECC_Pawn" "ECR_Ignore")
      (`PrimitiveComponent.SetCollisionResponseToChannel` _capsulecomponent "ECC_Camera" "ECR_Ignore")
      (`PrimitiveComponent.SetPhysicsLinearVelocity` (`self.Mesh`) (* (`KismetMathLibrary.Normal` (`self.K2_GetActorLocation` DamageCauser)) 10000.0) true "None")
      (`KismetSystemLibrary.Delay` 0.4)
      (`self.K2_DestroyActor`))))

(fn `UserConstructionScript`)