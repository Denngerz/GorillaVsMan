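; AI controller for human characters that runs the BT_Human behavior tree and feeds it sight of the player.
; Perception updates go to ProcessSightSense, which ignores everything except sight stimuli from player 0's character.
; Sighting the player sets the TargetActor blackboard key.
; Losing sight clears TargetActor and saves the player's actual location at that moment, rather than the stimulus location, as LastKnownLocation.
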(event `self.ReceiveBeginPlay`
  (`self.RunBehaviorTree` "/Game/Blueprints/Human/BT_Human.BT_Human"))

(event `self.AIPerception.OnTargetPerceptionUpdated`
  (params (Actor :type "Actor Object Reference") (Stimulus :type "AIStimulus Structure"))
  (`self.ProcessSightSense` Actor Stimulus))

(fn `ProcessSightSense`
  (params (Actor :type "Object Object Reference") (Stimulus :type "AIStimulus Structure (by ref)"))
  (bind (_stimulus_age _stimulus_expirationage _stimulus_strength _stimulus_stimuluslocation _stimulus_receiverlocation _stimulus_tag _stimulus_bsuccessfullysensed) (break `AIStimulus` (`local.Stimulus`)))
  (bind _returnvalue (`AIPerceptionSystem.GetSenseClassForStimulus` Stimulus))
  (if (== _returnvalue "/Script/AIModule.AISense_Sight")
    (if (== (`local.Actor`) (`GameplayStatics.GetPlayerCharacter` 0))
      (if _stimulus_bsuccessfullysensed
        (`BlackboardComponent.SetValueAsObject` (`self.Blackboard`) "TargetActor" (`GameplayStatics.GetPlayerCharacter` 0))
        (else
          (`BlackboardComponent.SetValueAsObject` (`self.Blackboard`) "TargetActor" null)
          (`BlackboardComponent.SetValueAsVector` (`self.Blackboard`) "LastKnownLocation" (`self.K2_GetActorLocation` (`GameplayStatics.GetPlayerCharacter` 0))))))))

(fn `UserConstructionScript`)